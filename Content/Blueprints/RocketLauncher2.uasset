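; Rocket launcher Blueprint that spawns and launches rocket projectiles from the player's camera.
; When CanFire is true, the Fire event spawns a RocketProjectile at ProjectileOffset rotated into camera space, matching the camera's rotation.
; It sends the rocket along the camera's forward vector, prints a debug message and calls StartCooldown, which is defined outside this graph.
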(event `self.ReceiveBeginPlay`)

(event `self.Fire`
  (bind (_returnvalue_location _returnvalue_rotation) (`KismetMathLibrary.BreakTransform` (`SceneComponent.K2_GetComponentToWorld` (`self.PlayerCam`))))
  (if (`self.CanFire`)
    (`KismetSystemLibrary.PrintString` "Fired!")
    (bind _returnvalue (`|SpawnActorFromClass` "/Game/Blueprints/Projectiles/RocketProjectile.RocketProjectile_C" (`KismetMathLibrary.MakeTransform` (+ (`KismetMathLibrary.GreaterGreater_VectorRotator` (`self.ProjectileOffset`) _returnvalue_rotation) _returnvalue_location) _returnvalue_rotation) "Undefined" "OverrideRootScale" null null))
    (`/Game/Blueprints/Projectiles/BaseProjectileBP.FireInDirection` _returnvalue (`SceneComponent.GetForwardVector` (`self.PlayerCam`)) null)
    (`self.StartCooldown`)))

(fn `UserConstructionScript`)