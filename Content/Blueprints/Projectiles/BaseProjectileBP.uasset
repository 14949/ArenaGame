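; Base projectile Blueprint that flies in a straight line once fired and destroys itself on hitting anything not tagged Player.
; FireInDirection enables movement, and Tick then calls FlyInDirection, which moves the actor by Direction times Speed using a swept SetActorLocation, without delta-time scaling.
; A valid Hit stops movement and fires the HitSomething dispatcher before destruction.
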(event `self.ReceiveHit`
  (params (MyComp :type "PrimitiveComponent Object Reference") (Other :type "Actor Object Reference") (OtherComp :type "PrimitiveComponent Object Reference") (bSelfMoved :type Boolean) (HitLocation :type "Vector Structure") (HitNormal :type "Vector Structure") (NormalImpulse :type "Vector Structure") (Hit :type "HitResult Structure (by ref)"))
  (`KismetSystemLibrary.PrintString` "Target hit")
  (if (not (`self.ActorHasTag` Other "Player"))
    (set `self.HasDirection` false)
    (`self.HitSomething`)
    (`self.K2_DestroyActor`)))

(event `self.ReceiveTick`
  (params (DeltaSeconds :type "Float (single-precision)"))
  (if (`self.HasDirection`)
    (`self.Fly In Direction` (stale `FireInDirection` Direction))))

(event `FireInDirection`
  (params (Direction :type "Vector Structure"))
  (set `self.HasDirection` true))

(fn `Fly In Direction`
  (params (Direction :type "Vector Structure"))
  (`self.K2_SetActorLocation` (+ (* Direction (`self.Speed`)) (`self.K2_GetActorLocation`)) true))

(fn `UserConstructionScript`)