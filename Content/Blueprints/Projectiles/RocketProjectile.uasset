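; Rocket projectile that explodes on impact, knocking back and damaging nearby characters.
; On the inherited hit event it spawns a radius-scaled explosion effect and sphere-overlaps Characters around the impact point.
; Knockback points away from the blast, weakens with distance up to a clamp, and uses separate Player and Enemy multipliers before LaunchCharacter.
; Launched characters tagged HasHealth take flat damage; debug sphere and lines are drawn.
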(event `self.ReceiveBeginPlay`
  (`parent.ReceiveBeginPlay`)
  (add `self.HitSomething` (delegate `HitSomething_Event`)))

(event `HitSomething_Event`
  (bind _returnvalue (`self.K2_GetActorLocation`))
  (bind _explosionradius (`self.ExplosionRadius`))
  (`GameplayStatics.SpawnEmitterAtLocation` "/Game/StarterContent/Particles/P_Explosion.P_Explosion" _returnvalue (struct) (`KismetMathLibrary.Conv_DoubleToVector` (* (`self.EffectScale`) (* (`self.ExplosionRadius`) 0.01))))
  (`KismetSystemLibrary.DrawDebugSphere` _returnvalue _explosionradius 12 (struct :`R` 1.0 :`G` 0.834575 :`B` 0.000243 :`A` 1.0) 6.0 1.0)
  (bind _outactors (`KismetSystemLibrary.SphereOverlapActors` _returnvalue _explosionradius (`self.Object Types`) "/Script/Engine.Character" (`|MakeArray` self :!type "Actor Object Reference")))
  (for _array_element _outactors
    (bind _direcationandmagnitude (`self.CalcKnockback` _returnvalue (`self.K2_GetActorLocation` _array_element)))
    (bind _ascharacter (cast `Character` _array_element))
    (if (`self.ActorHasTag` _ascharacter "Player")
      (`Character.LaunchCharacter` _ascharacter (* _direcationandmagnitude (`self.PlayerKnockbackMod`)) false false)
      (`KismetSystemLibrary.DrawDebugLine` _returnvalue (+ _returnvalue _direcationandmagnitude) (struct :`R` 0.9125 :`B` 0.014283 :`A` 1.0) 4.0 1.0 :!label _label)
      ;[1 1 1] Damage Area
      (if (`self.ActorHasTag` _array_element "HasHealth")
        (`/Game/Components/Health.Damage` (`self.GetComponentByClass` _array_element "/Game/Components/Health.Health_C") (`self.Damage`)))
      (elif (`self.ActorHasTag` _ascharacter "Enemy")
        (`Character.LaunchCharacter` _ascharacter (* _direcationandmagnitude (`self.EnemyKnockbackMod`)) false false)
        (goto _label)))))

(fn `CalcKnockback`
  (params (ExplosionPosition :type "Vector Structure") (ActorPosition :type "Vector Structure"))
  (returns (DirecationAndMagnitude :type "Vector Structure"))
  (return (* (* (`KismetMathLibrary.Normal` (- ActorPosition ExplosionPosition)) (`KismetMathLibrary.FClamp` (- (`self.ExplosionRadius`) (`KismetMathLibrary.Vector_Distance` ExplosionPosition ActorPosition)) 0.0 (`self.MaxKnockback`))) (`self.KnockbackPower`))))

(fn `UserConstructionScript`
  (`parent.UserConstructionScript`))