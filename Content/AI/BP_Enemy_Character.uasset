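; BP_Enemy_Character is an AI enemy character that awards score to the player when it dies.
; On BeginPlay it caches the first-person player character; the Health component's Death event adds ScoreValue to that player and destroys the enemy.
; Helper functions set the movement component's max walk speed and fire the held weapon if one is valid.
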(event `self.ReceiveBeginPlay`
  (bind _asbp_first_person_character (cast `/Game/FirstPerson/Blueprints/BP_FirstPersonCharacter` (`GameplayStatics.GetPlayerCharacter` 0)))
  (set `self.Player` _asbp_first_person_character))

(event `self.Health.OnDamageTaken`)

(event `self.Health.Death`
  (`/Game/FirstPerson/Blueprints/BP_FirstPersonCharacter.AddScore` (`self.Player`) (`self.ScoreValue`))
  (`self.K2_DestroyActor`))

(fn `FireWeapon`
  (if (`KismetSystemLibrary.IsValid` (`self.HeldWeapon`))
    (`WeaponBase.Fire` (`self.HeldWeapon`))))

(fn `UpdateWalkSpeed`
  (params (NewWalkSpeed :type "Float (double-precision)"))
  (set `CharacterMovementComponent.MaxWalkSpeed` NewWalkSpeed (`self.CharacterMovement`)))

(fn `UserConstructionScript`)