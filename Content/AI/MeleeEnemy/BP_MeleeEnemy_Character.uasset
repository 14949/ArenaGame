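; Melee enemy AI character that attacks with a Fists child actor as its held weapon.
; On BeginPlay it stores the fists as HeldWeapon and caches its AI Blackboard.
; Each tick it sets the Attacking flag on its AB_Ninja animation instance when the Blackboard reports IsInAttackRange and no attack is already running, so the animation Blueprint drives the attack.
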(event `self.ReceiveBeginPlay`
  (`parent.ReceiveBeginPlay`)
  (bind _asfists (cast `/Game/AI/Fists` (`ChildActorComponent.ChildActor` (`self.Fists`))))
  (set `self.HeldWeapon` _asfists)
  (set `self.Blackboard` (`AIBlueprintHelperLibrary.GetBlackboard` null)))

(event `self.ReceiveTick`
  (params (DeltaSeconds :type "Float (single-precision)"))
  (`self.UpdateAttackingOnAnimation`))

(fn `UserConstructionScript`
  (`parent.UserConstructionScript`))